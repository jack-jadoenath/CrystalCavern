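; BP_Cannon is a cannon actor that automatically fires BP_Projectile actors in an endless loop from BeginPlay.
; Each cycle waits for FireRate, then spawns a projectile at ProjectileComponent's location and rotation, scaled by ProjectileScale.
; A timeline then slides CannonBarrel along its local Y axis, and its Cannon Fired event track restarts the cycle.
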(event `self.ReceiveBeginPlay`
  (`KismetSystemLibrary.Delay` (`self.Fire Rate`) :!label _label)
  (`self.Spawn Projectile`)
  (bind (_direction _barrel_location) (`Timeline|Barrel Animation Timeline` :!via `PlayFromStart`)
    (:`Update`
      (`self.Move Cannon Barrel` _barrel_location))
    (:`Cannon Fired`
      (goto _label))))

(fn `Move Cannon Barrel`
  (params (`Barrel Y Location` :type "Float (double-precision)"))
  (`SceneComponent.K2_SetRelativeLocation` (`self.Cannon_Barrel`) (`KismetMathLibrary.MakeVector` 0.0 `Barrel Y Location`) false false))

(fn `Spawn Projectile`
  (bind _projectile_component (`self.Projectile Component`))
  (`|SpawnActorFromClass` "/Game/CavernGame/Blueprints/Actor/Projectiles/BP_Projectile.BP_Projectile_C" (`KismetMathLibrary.MakeTransform` (`SceneComponent.K2_GetComponentLocation` _projectile_component) (`SceneComponent.K2_GetComponentRotation` _projectile_component) (`KismetMathLibrary.Conv_DoubleToVector` (`self.Projectile Scale`))) "AdjustIfPossibleButAlwaysSpawn" "OverrideRootScale" null null))

(fn `UserConstructionScript`)