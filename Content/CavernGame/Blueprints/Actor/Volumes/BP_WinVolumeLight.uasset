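; Level exit volume that lets the player finish a cavern level once no BP_Crystal actors remain.
; It creates the CrystalHud widget on BeginPlay and polls every Tick for remaining crystals, turning its point light green when none are left.
; A player overlap then opens the next level in the LevelNames array, found from the current level's index, or quits the game on the final entry.
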(event `self.ReceiveBeginPlay`
  (bind _returnvalue (`|CreateWidget` "/Game/CavernGame/UI/HUD/CrystalHud.CrystalHud_C"))
  (`UserWidget.AddToViewport` _returnvalue 0))

(event `self.ReceiveActorBeginOverlap`
  (params (OtherActor :type "Actor Object Reference"))
  (`/Game/CavernGame/Blueprints/Libs/CM_MacroLibrary.IsPlayer` OtherActor
    (:`IsPlayer`
      (if (not (`self.Any Crystals Remaining`))
        (`self.Complete Level`)))))

(event `self.ReceiveTick`
  (params (DeltaSeconds :type "Float (single-precision)"))
  (if (not (`self.Any Crystals Remaining`))
    (`LightComponent.SetLightColor` (`self.PointLight`) (struct :`R` 0.003433 :`G` 0.807292 :`A` 1.0) true)))

(fn `Any Crystals Remaining`
  (returns (`Return Value` :type Boolean))
  (bind _outactors (`GameplayStatics.GetAllActorsOfClass` "/Game/CavernGame/Blueprints/Actor/Collectables/BP_Crystal.BP_Crystal_C"))
  (return (> (`KismetArrayLibrary.Array_Length` _outactors) 0)))

(fn `Complete Level`
  (if (`self.Is Final Level?`)
    (`KismetSystemLibrary.QuitGame` null "Quit")
    (else
      (`self.Load Next Level`))))

(fn `Get Current Level Index`
  (returns (ReturnValue :type Integer))
  (bind _returnvalue (`GameplayStatics.GetCurrentLevelName` true))
  (return (`KismetArrayLibrary.Array_Find` (`self.Level Names`) (`KismetStringLibrary.Conv_StringToName` _returnvalue))))

(fn `Get Next Level Name`
  (returns (Output :type Name))
  (bind _result (`/Engine/EditorBlueprintResources/StandardMacros.IncrementInt` (`self.Get Current Level Index`))
    (:`  `
      (return (`|GetArrayItem` (`self.Level Names`) _result)))))

(fn `Is Final Level?`
  (returns (`Return Value` :type Boolean))
  (return (== (`KismetArrayLibrary.Array_LastIndex` (`self.Level Names`)) (`self.Get Current Level Index`))))

(fn `Load Next Level`
  (`GameplayStatics.OpenLevel` (`self.Get Next Level Name`)))

(fn `UserConstructionScript`)