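; BP_TeleportVolumeLight is a volume actor that instantly moves the player pawn to TargetLocation, without sweeping, when the player overlaps it.
; The overlap event filters through IsPlayer, then teleports player pawn 0.
; It also defines helpers for checking remaining BP_Crystal actors and advancing through LevelNames or quitting on the final level, but the overlap event calls none of them.
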(event `self.ReceiveActorBeginOverlap`
  (params (OtherActor :type "Actor Object Reference"))
  (`/Game/CavernGame/Blueprints/Libs/CM_MacroLibrary.IsPlayer` OtherActor
    (:`IsPlayer`
      (`self.K2_SetActorLocation` (`GameplayStatics.GetPlayerPawn` 0) (`self.TargetLocation`) false true))))

(fn `Any Crystals Remaining`
  (returns (`Return Value` :type Boolean))
  (bind _outactors (`GameplayStatics.GetAllActorsOfClass` "/Game/CavernGame/Blueprints/Actor/Collectables/BP_Crystal.BP_Crystal_C"))
  (return (> (`KismetArrayLibrary.Array_Length` _outactors) 0)))

(fn `Complete Level`
  (if (`self.Is Final Level?`)
    (`KismetSystemLibrary.QuitGame` null "Quit")
    (else
      (`self.Load Next Level`))))

(fn `Get Current Level Index`
  (returns (ReturnValue :type Integer))
  (bind _returnvalue (`GameplayStatics.GetCurrentLevelName` true))
  (return (`KismetArrayLibrary.Array_Find` (`self.Level Names`) (`KismetStringLibrary.Conv_StringToName` _returnvalue))))

(fn `Get Next Level Name`
  (returns (Output :type Name))
  (bind _result (`/Engine/EditorBlueprintResources/StandardMacros.IncrementInt` (`self.Get Current Level Index`))
    (:`  `
      (return (`|GetArrayItem` (`self.Level Names`) _result)))))

(fn `Is Final Level?`
  (returns (`Return Value` :type Boolean))
  (return (== (`KismetArrayLibrary.Array_LastIndex` (`self.Level Names`)) (`self.Get Current Level Index`))))

(fn `Load Next Level`
  (`GameplayStatics.OpenLevel` (`self.Get Next Level Name`)))

(fn `UserConstructionScript`)