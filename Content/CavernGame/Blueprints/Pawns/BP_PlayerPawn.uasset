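; BP_PlayerPawn is the player pawn for CavernGame, a sphere rolled by input-driven torque that restarts the level when damaged.
; The forward/backward axis applies acceleration-scaled torque on both X and Y of SMSphere, while the right/left axis event is empty.
; BeginPlay fades the camera in from black.
; The first damage event fades to black and reopens the current level after the fade; R restarts immediately.
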(event `self.ReceiveBeginPlay`
  (`PlayerCameraManager.StartCameraFade` (`GameplayStatics.GetPlayerCameraManager` 0) 1.0 0.0 (`self.Fade Out In Seconds`) (struct :`A` 1.0) false true))

(event `InputAxis|Move Right/Left`
  (params (AxisValue :type "Float (single-precision)")))

(event `InputAxis|Move Forward/Backwards`
  (params (AxisValue :type "Float (single-precision)"))
  (`PrimitiveComponent.AddTorqueInRadians` (`self.SM_Sphere`) (`KismetMathLibrary.MakeVector` (* (stale `InputAxis|Move Right/Left` AxisValue) (`self.Accelration`)) (* AxisValue (`self.Accelration`))) "None" true))

(event `Key|R`
  (params (Key :type "Key Structure"))
  (:`Pressed`
    (`self.Restart Current Level`)))

(event `self.ReceiveAnyDamage`
  (params (Damage :type "Float (single-precision)") (DamageType :type "DamageType Object Reference") (InstigatedBy :type "Controller Object Reference") (DamageCauser :type "Actor Object Reference"))
  (`/Engine/EditorBlueprintResources/StandardMacros.DoOnce` false
    (:`Completed`
      (bind _delay_and_fade_seconds (`self.Camera Fade Start`))
      (`KismetSystemLibrary.Delay` _delay_and_fade_seconds)
      (`self.Restart Current Level`))))

(fn `Camera Fade Start`
  (returns (`Delay and Fade Seconds` :type "Float (double-precision)"))
  (bind _delay_and_fade_seconds (`self.Delay and Fade Seconds`))
  (`PlayerCameraManager.StartCameraFade` (`GameplayStatics.GetPlayerCameraManager` 0) 0.0 1.0 _delay_and_fade_seconds (struct :`A` 1.0) false true)
  (return _delay_and_fade_seconds))

(fn `Restart Current Level`
  (bind _returnvalue (`GameplayStatics.GetCurrentLevelName` true))
  (`GameplayStatics.OpenLevel` (`KismetStringLibrary.Conv_StringToName` _returnvalue)))

(fn `UserConstructionScript`)